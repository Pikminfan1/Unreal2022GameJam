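; A turret projectile sphere that knocks the player character away on contact.
; On overlap with BP_PlayerCharacter it launches the character along LaunchDirection rotated by its own rotation, scaled by LaunchForce and overriding existing velocity, then destroys itself.
; Overlaps with Turret_BP1 are ignored, while any other overlap destroys it.
; It also destroys itself after an InitialLifeSpan delay from BeginPlay.
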(event Collision|EventActorBeginOverlap
  (params (OtherActor :type Actor%20Object%20Reference))
  (bind _asbp_player_character (Utilities|Casting|CastToBP_PlayerCharacter OtherActor)
    (:then
      (CallFunction|LaunchPlayer _asbp_player_character))
    (:CastFailed
      (Utilities|Casting|CastToTurret_BP1 OtherActor
        (:CastFailed
          _))))
  (Actor|DestroyActor))

(event EventTick
  (params (DeltaSeconds :type Float%20%28single-precision%29)))

(event EventBeginPlay
  (Utilities|FlowControl|Delay (Variables|Actor|GetInitialLifeSpan))
  (Actor|DestroyActor))

(fn ConstructionScript)

(fn LaunchPlayer
  (params (Player%20Character :type Unreal%202022%20Game%20Jam%20Character%20Object%20Reference))
  (Character|LaunchCharacter Player%20Character (* (Math|Vector|Normalize (Math|Vector|RotateVector (Variables|Default|GetLaunchDirection) (Transformation|GetActorRotation self))) (Variables|Default|GetLaunchForce)) true true))
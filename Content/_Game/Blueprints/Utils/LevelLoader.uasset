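; LevelLoader is a trigger actor that completes the level when BP_PlayerCharacter overlaps it.
; On overlap it flags the player's level as complete and swaps the HUD for a UMG_LevelComplete widget.
; It then ignores move input, switches to UI-only input with a visible cursor and stops the BP_GameMode counter.
; Despite the name it loads no level: the CanLoadNextLevel branch is empty and LevelToLoad is unused.
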(event EventBeginPlay)

(event Collision|EventActorBeginOverlap
  (params (OtherActor :type Actor%20Object%20Reference))
  (bind _returnvalue (Game|GetPlayerController 0))
  (bind _asbp_player_character (Utilities|Casting|CastToBP_PlayerCharacter OtherActor))
  (Variables|/Game/_Game/Blueprints/Player/BP_PlayerCharacter.BP_PlayerCharacter_C|SetbIsLevelComplete _asbp_player_character true)
  (Widget|RemovefromParent (Variables|/Game/_Game/Blueprints/Player/BP_PlayerCharacter.BP_PlayerCharacter_C|GetHUD_WBP _asbp_player_character))
  (bind _returnvalue_2 (UserInterface|CreateWidget "/Game/_Game/UI/UMG_LevelComplete.UMG_LevelComplete_C"))
  (UserInterface|Viewport|AddtoViewport _returnvalue_2 0)
  (Input|SetIgnoreMoveInput _returnvalue true)
  (Input|SetInputModeUIOnly _returnvalue 0 "DoNotLock")
  (Variables|/Script/Engine.PlayerController|SetbShowMouseCursor _returnvalue true)
  (bind _asbp_game_mode (Utilities|Casting|CastToBP_GameMode (Game|GetGameMode)))
  (Variables|/Game/_Game/Blueprints/BP_GameMode.BP_GameMode_C|SetCounterActive _asbp_game_mode false)
  (if (Variables|Default|GetbCanLoadNextLevel)
    _))

(event EventTick
  (params (DeltaSeconds :type Float%20%28single-precision%29)))

(fn ConstructionScript)
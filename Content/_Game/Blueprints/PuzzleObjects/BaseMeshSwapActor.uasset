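; BaseMeshSwapActor is a puzzle-object actor that switches its static mesh's look between Heaven and Hell by swapping the first material slot.
; On BeginPlay it caches BP_GameMode and starts a fast looping timer.
; The timer polls the game mode's IsHell flag and reapplies the matching material on every call, whether or not the state has changed.
; Despite the name, only the material changes, not the mesh.
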(event Custom|SetHell
  (Rendering|Material|SetMaterial (Variables|Default|GetStaticMesh) 0 (Variables|Default|GetHellMat)))

(event Custom|SetHeaven
  (Rendering|Material|SetMaterial (Variables|Default|GetStaticMesh) 0 (Variables|Default|GetHeavenMat)))

(event Custom|CheckSwitch
  (if (Variables|/Game/_Game/Blueprints/BP_GameMode.BP_GameMode_C|GetbIsHell (Variables|Default|GetAs%20BP%20Game%20Mode))
    (CallFunction|SetHell)
    (else
      (CallFunction|SetHeaven))))

(event EventBeginPlay
  (Utilities|Time|SetTimerbyEvent (delegate Custom|CheckSwitch) 0.1 true)
  (bind _asbp_game_mode (Utilities|Casting|CastToBP_GameMode (Game|GetGameMode)))
  (Variables|Default|SetAs%20BP%20Game%20Mode _asbp_game_mode))

(event Collision|EventActorBeginOverlap
  (params (OtherActor :type Actor%20Object%20Reference)))

(event EventTick
  (params (DeltaSeconds :type Float%20%28single-precision%29)))

(fn ConstructionScript)
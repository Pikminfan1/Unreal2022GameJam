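; Launch pad puzzle object that flings the player character when they overlap it.
; On overlap it rotates a local launch direction by the actor's rotation, normalizes it and scales it by a force magnitude.
; The result overrides the character's velocity through LaunchCharacter, then a Wwise bounce sound plays on the character and its double jump count is set to one.
; A debug print of the direction remains active.
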(event EventBeginPlay)

(event Collision|EventActorBeginOverlap
  (params (OtherActor :type Actor%20Object%20Reference))
  (bind _self self)
  (bind _launchdirection (Variables|Default|GetLaunchDirection))
  (bind _forcemagnitude (Variables|Default|GetForceMagnitude))
  (bind _returnvalue (Transformation|GetActorRotation _self))
  (bind _returnvalue_2 (Math|Vector|RotateVector _launchdirection _returnvalue))
  (bind _returnvalue_3 (Math|Vector|Normalize _returnvalue_2))
  (bind _asunreal_2022game_jam_character (Utilities|Casting|CastToUnreal2022GameJamCharacter OtherActor))
  (Development|PrintString (Utilities|String|ToString(Vector) _returnvalue_3))
  (Character|LaunchCharacter _asunreal_2022game_jam_character (* _returnvalue_3 (Math|Vector|MakeVector _forcemagnitude _forcemagnitude _forcemagnitude)) true true)
  (Class|AkGameplayStatics|PostEvent "/Game/_Game/Audio/Events/Play_Bounce.Play_Bounce" _asunreal_2022game_jam_character)
  (Class|Unreal2022GameJamCharacter|SetCurrentDoubleJumpCount _asunreal_2022game_jam_character 1))

(event EventTick
  (params (DeltaSeconds :type Float%20%28single-precision%29)))

(fn ConstructionScript)
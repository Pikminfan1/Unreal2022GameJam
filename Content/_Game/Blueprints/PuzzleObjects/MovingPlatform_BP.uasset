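; MovingPlatform_BP is a puzzle object platform that travels between a home location and a travel-to location.
; The construction script gives an InterpToMovement component two relative control points and a travel Duration from the instance's variables.
; On BeginPlay, IsMoving decides whether that component ticks.
; Toggleon and ToggleOff events start or pause the motion by enabling or disabling the component's tick.
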(event EventBeginPlay
  (bind _interptomovement (Variables|Default|GetInterpToMovement))
  (if (Variables|Default|GetbIsMoving)
    (Components|Tick|SetComponentTickEnabled _interptomovement true)
    (else
      (Components|Tick|SetComponentTickEnabled _interptomovement false))))

(event EventToggleon
  (Components|Tick|SetComponentTickEnabled (Variables|Default|GetInterpToMovement) true))

(event EventToggleOff
  (Components|Tick|SetComponentTickEnabled (Variables|Default|GetInterpToMovement) false))

(fn ConstructionScript
  (bind _interptomovement (Variables|Default|GetInterpToMovement))
  (Variables|/Script/Engine.InterpToMovementComponent|SetControlPoints _interptomovement (Utilities|Array|MakeArray (Utilities|Struct|MakeInterpControlPoint (Variables|Default|GetHomeLocation) true) (Utilities|Struct|MakeInterpControlPoint (Variables|Default|GetTravelToLocation) true)))
  (Variables|/Script/Engine.InterpToMovementComponent|SetDuration _interptomovement (Variables|Default|GetDuration)))
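; Launch pad puzzle object that is solid in the Hell state and passable in the Heaven state.
; SetHell applies the opaque hell material to the cube and enables query and physics collision on cube and box.
; SetHeaven applies the translucent material and disables that collision, with paired flags skipping repeated swaps.
; BeginPlay and overlap only call the parent, and no launch logic appears in this graph.
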(event EventBeginPlay
  (|CallParentFunction))

(event Collision|EventActorBeginOverlap
  (params (OtherActor :type Actor%20Object%20Reference))
  (|CallParentFunction OtherActor))

(event EventTick
  (params (DeltaSeconds :type Float%20%28single-precision%29))
  (|CallParentFunction DeltaSeconds) ; This node is disabled and will not be called.\nDrag off pins to build functionality.
)

(event EventSetHell
  (if (not (Variables|Default|GetbHasSwappedHell))
    (Rendering|Material|SetMaterial (Variables|Default|GetCube) 0 "/Game/_Game/Materials/M_HellMaterial_Opaque.M_HellMaterial_Opaque")
    (Collision|SetCollisionEnabled (Variables|Default|GetBox) "QueryAndPhysics")
    (Variables|Default|SetbHasSwappedHell true)
    (Variables|Default|SetbHasSwappedHeaven false)))

(event EventSetHeaven
  (if (not (Variables|Default|GetbHasSwappedHeaven))
    (Rendering|Material|SetMaterial (Variables|Default|GetCube) 0 "/Game/_Game/Materials/M_HellMaterial_Trans.M_HellMaterial_Trans")
    (Collision|SetCollisionEnabled (Variables|Default|GetBox) "NoCollision")
    (Variables|Default|SetbHasSwappedHeaven true)
    (Variables|Default|SetbHasSwappedHell false)))

(fn ConstructionScript
  (|CallParentFunction))
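; Base launch pad puzzle object that swaps its cube's material between Heaven and Hell looks.
; A looping timer started on BeginPlay polls the IsHell flag on BP_GameMode and calls SetHell or SetHeaven.
; Each applies its material unless its HasSwapped flag is set, though neither sets that flag here.
; Overlap handling is left to the parent class.
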(event Custom|SetHell
  (if (not (Variables|Default|GetbHasSwappedHell))
    (Rendering|Material|SetMaterial (Variables|Default|GetCube) 0 (Variables|Default|GetHellMat))))

(event Custom|SetHeaven
  (if (not (Variables|Default|GetbHasSwappedHeaven))
    (Rendering|Material|SetMaterial (Variables|Default|GetCube) 0 (Variables|Default|GetHeavenMat))))

(event Custom|CheckSwitch
  (if (Variables|/Game/_Game/Blueprints/BP_GameMode.BP_GameMode_C|GetbIsHell (Variables|Default|GetAs%20BP%20Game%20Mode))
    (CallFunction|SetHell)
    (else
      (CallFunction|SetHeaven))))

(event EventBeginPlay
  (Utilities|Time|SetTimerbyEvent (delegate Custom|CheckSwitch) 0.1 true)
  (bind _asbp_game_mode (Utilities|Casting|CastToBP_GameMode (Game|GetGameMode)))
  (Variables|Default|SetAs%20BP%20Game%20Mode _asbp_game_mode)
  (|CallParentFunction))

(event Collision|EventActorBeginOverlap
  (params (OtherActor :type Actor%20Object%20Reference))
  (|CallParentFunction OtherActor))

(event EventTick
  (params (DeltaSeconds :type Float%20%28single-precision%29))
  (|CallParentFunction DeltaSeconds) ; This node is disabled and will not be called.\nDrag off pins to build functionality.
)

(fn ConstructionScript
  (|CallParentFunction))
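; HeavenBlock_BP is a puzzle block that is solid in the Heaven state and passable in the Hell state.
; SetHeaven enables query and physics collision on the static mesh and applies the opaque Heaven material.
; SetHell disables that collision and swaps to the translucent Heaven material.
; The block has no active logic of its own beyond these two events, so the state switch is triggered from outside this graph.
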(event EventBeginPlay
  (|CallParentFunction) ; This node is disabled and will not be called.\nDrag off pins to build functionality.
)

(event Collision|EventActorBeginOverlap
  (params (OtherActor :type Actor%20Object%20Reference))
  (|CallParentFunction OtherActor) ; This node is disabled and will not be called.\nDrag off pins to build functionality.
)

(event EventTick
  (params (DeltaSeconds :type Float%20%28single-precision%29))
  (|CallParentFunction DeltaSeconds) ; This node is disabled and will not be called.\nDrag off pins to build functionality.
)

(event EventSetHell
  (bind _staticmesh (Variables|Default|GetStaticMesh))
  (Collision|SetCollisionEnabled _staticmesh "NoCollision")
  (Rendering|Material|SetMaterial _staticmesh 0 "/Game/_Game/Materials/M_HeavenMaterial_Trans.M_HeavenMaterial_Trans"))

(event EventSetHeaven
  (bind _staticmesh (Variables|Default|GetStaticMesh))
  (Collision|SetCollisionEnabled _staticmesh "QueryAndPhysics")
  (Rendering|Material|SetMaterial _staticmesh 0 "/Game/_Game/Materials/M_HeavenMaterial_Opaque.M_HeavenMaterial_Opaque"))

(fn ConstructionScript
  (|CallParentFunction))
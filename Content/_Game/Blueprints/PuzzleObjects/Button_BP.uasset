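; Pressure-plate style puzzle button that switches a linked ToggleActor on while an actor overlaps it.
; Begin overlap calls ToggleOn and moves the Cylinder down from the relative home position stored at BeginPlay; end overlap calls ToggleOff and moves it back.
; Overlaps are neither filtered nor counted, so any actor leaving turns the target off, and each event prints the other actor's name.
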(event EventBeginPlay
  (Variables|Default|SetHomePosition (Variables|/Script/Engine.SceneComponent|GetRelativeLocation (Variables|Default|GetCylinder))))

(event Collision|EventActorEndOverlap
  (params (OtherActor :type Actor%20Object%20Reference))
  (Default|ToggleOff (Variables|Default|GetToggleActor))
  (Development|PrintString (Utilities|GetDisplayName OtherActor))
  (Components|MoveComponentTo (Variables|Default|GetCylinder) (Variables|Default|GetHomePosition) "0, 0, 0" false false 0.2 false))

(event Collision|EventActorBeginOverlap
  (params (OtherActor :type Actor%20Object%20Reference))
  (Default|Toggleon (Variables|Default|GetToggleActor))
  (Development|PrintString (Utilities|GetDisplayName OtherActor))
  (Components|MoveComponentTo (Variables|Default|GetCylinder) (- (Variables|Default|GetHomePosition) "0,0,5.000000") "0, 0, 0" false false 0.2 false))

(event EventTick
  (params (DeltaSeconds :type Float%20%28single-precision%29)))

(fn ConstructionScript)
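; BP_Player is the player character Blueprint, delegating parkour movement and object pickup to its ParkourMovement and PickupComponent components.
; It initializes both with itself on BeginPlay, then forwards jump and landing events to ParkourMovement alongside the standard Jump.
; Interact toggles between pickup and drop through the IsHoldingObject flag, which is set after PickupObject without checking whether anything was grabbed.
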(event EventBeginPlay
  (bind _self self)
  (Utilities|FlowControl|Sequence
    (:then_0
      (Default|Initialize (Variables|Default|GetParkourMovement) _self)
      (Default|Initialize (Variables|Default|GetPickupComponent) _self))))

(event EventOnLanded
  (params (Hit :type Hit%20Result%20Structure%20%28by%20ref%29))
  (Default|LandEvent (Variables|Default|GetParkourMovement)))

(event Input|ActionEvents|InputActionJump
  (params (Key :type Key%20Structure :default "None"))
  (:Pressed
    (Character|Jump)
    (Default|JumpEvent (Variables|Default|GetParkourMovement))))

(event Input|ActionEvents|InputActionInteract
  (params (Key :type Key%20Structure :default "None"))
  (:Pressed
    (if (Variables|Default|GetbIsHoldingObject)
      (Default|DropObject (Variables|Default|GetPickupComponent))
      (Variables|Default|SetbIsHoldingObject false)
      (else
        (Default|PickupObject (Variables|Default|GetPickupComponent))
        (Variables|Default|SetbIsHoldingObject true)))))

(fn ConstructionScript)
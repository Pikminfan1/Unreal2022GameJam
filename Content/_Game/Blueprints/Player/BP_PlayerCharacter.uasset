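; Player character for a parkour game with a switchable Hell dimension, where the angel or devil mesh shows according to the game mode's state.
; BeginPlay initializes the parkour, pickup and sound components, takes the respawn point from a PlayerStart, hides both meshes' legs and creates the HUD.
; Inputs drive jumping, pickup/drop and dimension switching, which updates game mode, music and mesh.
; Tick drives footsteps, landing notifies parkour, and Respawn teleports back with Wwise death audio.
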(event Custom|Respawn
  ;[1 1 1] Respawn Player and Play SFX
  (Class|AkGameplayStatics|PostEvent "/Game/_Game/Audio/Events/Play_Player_Death.Play_Player_Death" self)
  (Transformation|SetActorLocation (Variables|Default|GetRespawnPoint) false false))

(event Custom|SwapMesh
  ;[1 1 1] Swap Visibility of Correct Mesh
  (if (Variables|/Game/_Game/Blueprints/BP_GameMode.BP_GameMode_C|GetbIsHell (Variables|Default|GetAs%20BP%20Game%20Mode))
    (Rendering|SetVisibility (Variables|Default|GetAngelMesh) true false)
    (Rendering|SetVisibility (Variables|Default|GetDevilMesh) false false)
    (else
      (Rendering|SetVisibility (Variables|Default|GetAngelMesh) false false)
      (Rendering|SetVisibility (Variables|Default|GetDevilMesh) true false))))

(event Custom|Hide%20Legs
  (bind _devilmesh (Variables|Default|GetDevilMesh))
  (bind _angelmesh (Variables|Default|GetAngelMesh))
  (Components|SkinnedMesh|HideBonebyName _angelmesh "angelgal_LeftUpLeg" "PBO_None")
  (Components|SkinnedMesh|HideBonebyName _angelmesh "angelgal_RightUpLeg" "PBO_None")
  (Components|SkinnedMesh|HideBonebyName _devilmesh "devildude_LeftUpLeg" "PBO_None")
  (Components|SkinnedMesh|HideBonebyName _devilmesh "devildude_RightUpLeg" "PBO_None"))

(event EventBeginPlay
  (bind _self self)
  (bind _parkourmovement (Variables|Default|GetParkourMovement))
  (bind _playersounds (Variables|Default|GetPlayerSounds))
  ;[1 1 1] Initialize
  (bind _asbp_game_mode (Utilities|Casting|CastToBP_GameMode (Game|GetGameMode)))
  (Utilities|FlowControl|Sequence
    (:then_0
      (Variables|Default|SetAs%20BP%20Game%20Mode _asbp_game_mode)
      ;;[1 1 1] Initialize Game Components
      (Default|Initialize _parkourmovement _self))
    (:then_1
      (Default|Initialize (Variables|Default|GetPickupComponent) _self))
    (:then_2
      ;;[1 1 1] Initialize Music Components
      (Default|Initialize _playersounds _self _parkourmovement (Variables|Default|GetAs%20BP%20Game%20Mode)))
    (:then_3
      (Default|SwitchMusicState _playersounds))
    (:then_4
      (Default|PlayMusic _playersounds))
    (:then_5
      ;;[1 1 1] Initialize Respawn By Looking for Player start in level
      (bind _outactors (Actor|GetAllActorsOfClass "/Script/Engine.PlayerStart"))
      (for _array_element _outactors
        (Variables|Default|SetRespawnPoint (Transformation|GetActorLocation _array_element))))
    (:then_6
      ;;[1 1 1] Initialize Starting Mesh
      (CallFunction|SwapMesh))
    (:then_7
      ;;[1 1 1] Mark Initialize as complete for other blueprints
      (Variables|Default|SetbIsInitialized true))
    (:then_8
      (CallFunction|HideLegs))
    (:then_9
      (bind _returnvalue (UserInterface|CreateWidget "/Game/_Game/UI/UMG_Hud.UMG_Hud_C" (Game|GetPlayerController 0)))
      (Variables|Default|SetHUD_WBP _returnvalue)
      (UserInterface|Viewport|AddtoViewport _returnvalue 0))
    (:then_10
      (Variables|Default|SetbIsLevelComplete false))))

(event EventOnLanded
  (params (Hit :type Hit%20Result%20Structure%20%28by%20ref%29))
  ;[1 1 1] Land Event For Parkour
  (Default|LandEvent (Variables|Default|GetParkourMovement)))

(event EventTick
  (params (DeltaSeconds :type Float%20%28single-precision%29))
  ;[1 1 1] Tick on Player Footsteps
  (Default|CallFootstepEvent (Variables|Default|GetPlayerSounds)))

(event Input|ActionEvents|InputActionJump
  (params (Key :type Key%20Structure :default "None"))
  ;[1 1 1] Jump and Play Jump SFX
  (:Pressed
    (Character|Jump)
    (Default|JumpEvent (Variables|Default|GetParkourMovement))
    (Default|PlayDoubleJumpSound (Variables|Default|GetPlayerSounds))))

(event Input|ActionEvents|InputActionInteract
  (params (Key :type Key%20Structure :default "None"))
  ;[1 1 1] Interact Action (unused?)
  (:Pressed
    (if (Variables|Default|GetbIsHoldingObject)
      (Default|DropObject (Variables|Default|GetPickupComponent))
      (Variables|Default|SetbIsHoldingObject false)
      (else
        (Default|PickupObject (Variables|Default|GetPickupComponent))
        (Variables|Default|SetbIsHoldingObject true)
        (Class|AkGameplayStatics|PostEvent "/Game/_Game/Audio/Events/Play_Pick_Up.Play_Pick_Up" self)))))

(event Input|ActionEvents|InputActionChangeState
  (params (Key :type Key%20Structure :default "None"))
  (bind _playersounds (Variables|Default|GetPlayerSounds))
  ;[1 1 1] Pass on Change state to components that need to listen for it
  (:Pressed
    (Utilities|FlowControl|Sequence
      (:then_0
        (Default|ChangeState (Variables|Default|GetAs%20BP%20Game%20Mode)))
      (:then_1
        (Default|PlayDimentonSwitchSound _playersounds))
      (:then_2
        (Default|SwitchMusicState _playersounds))
      (:then_3
        (CallFunction|SwapMesh)))))

(fn ConstructionScript)
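; BP_GameMode is a game mode that tracks play time and holds an IsHell world-state flag.
; While CounterActive, set on BeginPlay, each Tick grows ElapsedTime by delta seconds and adds that cumulative value, not the frame delta, to TotalTime on GameInstance_BP.
; The ChangeState event toggles IsHell.
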(event Custom|ChangeState
  (Variables|Default|SetbIsHell (not (Variables|Default|GetbIsHell))))

(event EventBeginPlay
  (Variables|Default|SetCounterActive true))

(event EventTick
  (params (DeltaSeconds :type Float%20%28single-precision%29))
  (if (Variables|Default|GetCounterActive)
    (bind _output_get (Variables|Default|SetElapsedTime (+ (Variables|Default|GetElapsedTime) DeltaSeconds)))
    (bind _asgame_instance_bp (Utilities|Casting|CastToGameInstance_BP (Game|GetGameInstance)))
    (Variables|/Game/_Game/Blueprints/Utils/GameInstance_BP.GameInstance_BP_C|SetTotalTime _asgame_instance_bp (+ (Variables|/Game/_Game/Blueprints/Utils/GameInstance_BP.GameInstance_BP_C|GetTotalTime _asgame_instance_bp) _output_get))))

(fn ConstructionScript)
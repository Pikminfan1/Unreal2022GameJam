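; Player sound component that plays Wwise footstep and double-jump audio for a parkour character.
; CallFootstepEvent starts a looping footstep timer during ground movement or wall running, choosing a faster interval if wall running at start, and clears it otherwise.
; Each step line-traces down, or toward a side-offset point when wall running, mapping the physical surface to a Default or Ice Wwise switch before posting the footstep event.
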(event Custom|Initialize
  (params (Character :type Unreal%202022%20Game%20Jam%20Character%20Object%20Reference) (ParkourMovement :type Parkour%20Movement%20Object%20Reference))
  ;[1 1 1] Footsteps
  (bind _output_get (Variables|Default|SetCharacter Character))
  (bind _output_get_2 (Variables|Default|SetParkourMovement ParkourMovement)))

(event Custom|PlayerFootstepSound
  ;[1 1 1] Footsteps
  (CallFunction|CheckSurfaceMaterial)
  (Class|AkGameplayStatics|PostEvent "/Game/Audio/Events/Play_FootstepsSwitch.Play_FootstepsSwitch" (Variables|Default|GetCharacter)))

(event Custom|CallFootstepEvent
  ;[1 1 1] Footsteps
  (if (and (or (>= (Math|Float|Absolute(Float) (.x (Pawn|Components|CharacterMovement|GetLastUpdateVelocity (Variables|/Script/Engine.Character|GetCharacterMovement (stale Custom|Initialize _output_get))))) 2.0) (>= (Math|Float|Absolute(Float) (.y (Pawn|Components|CharacterMovement|GetLastUpdateVelocity (Variables|/Script/Engine.Character|GetCharacterMovement (stale Custom|Initialize _output_get))))) 2.0)) (or (AI|Components|NavMovement|IsMovingonGround (Variables|/Script/Engine.Character|GetCharacterMovement (Variables|Default|GetCharacter))) (Variables|/Game/_Game/Blueprints/Components/ParkourMovement.ParkourMovement_C|GetWallRunning (stale Custom|Initialize _output_get_2))))
    (Utilities|FlowControl|DoOnce false :!label _label
      (:Completed
        (if (Variables|/Game/_Game/Blueprints/Components/ParkourMovement.ParkourMovement_C|GetWallRunning (Variables|Default|GetParkourMovement)) ; Change step speed depending on wall run state
          (Variables|Default|SetStepSpeed 0.3)
          (else
            (Variables|Default|SetStepSpeed 0.4)))
        (bind _returnvalue (Utilities|Time|SetTimerbyEvent (delegate Custom|PlayerFootstepSound) (Variables|Default|GetStepSpeed) true))))
    (else
      (Utilities|Time|ClearandInvalidateTimerbyHandle _returnvalue)
      (goto _label Reset))))

(event Custom|CheckSurfaceMaterial
  (bind _character (Variables|Default|GetCharacter))
  (bind _charactermovement (Variables|/Script/Engine.Character|GetCharacterMovement _character))
  (bind _returnvalue (Class|CharacterMovementComponent|GetLastUpdateLocation _charactermovement))
  ;[1 1 1] Checking Surface Material For Footstep Sound
  (if (Variables|/Game/_Game/Blueprints/Components/ParkourMovement.ParkourMovement_C|GetWallRunning (Variables|Default|GetParkourMovement))
    (if (Variables|/Game/_Game/Blueprints/Components/ParkourMovement.ParkourMovement_C|GetWallRunningOnLeft (Variables|Default|GetParkourMovement)) ; if player is wall running line trace to the wall running side
      (bind (_outhit _returnvalue_2) (Collision|LineTraceByChannel _returnvalue (+ (Math|Vector|GetRightVector (Math|Conversions|RotationFromXVector _returnvalue)) "-100.000000,0,0") "TraceTypeQuery1" false 0 "None")) ; trace to the left
      (if _returnvalue_2
        (CallFunction|SetSurfaceSwitch (Collision|GetSurfaceType _outhit)))
      (else
        (bind (_outhit_2 _returnvalue_3) (Collision|LineTraceByChannel _returnvalue (+ (Math|Vector|GetRightVector (Math|Conversions|RotationFromXVector _returnvalue)) "100.000000,0,0") "TraceTypeQuery1" false 0 "None")) ; trace to the right
        (if _returnvalue_3
          (CallFunction|SetSurfaceSwitch (Collision|GetSurfaceType _outhit_2)))))
    (else
      (bind (_outhit_3 _returnvalue_4) (Collision|LineTraceByChannel _returnvalue (- _returnvalue "0,0,1000.000000") "TraceTypeQuery1" false 0 "None")) ; If not wall running, line trace down
      (if _returnvalue_4
        (CallFunction|SetSurfaceSwitch (Collision|GetSurfaceType _outhit_3))))))

(event Custom|SetSurfaceSwitch
  (params (Selection :type EPhysicalSurface%20Enum :default "SurfaceType_Default"))
  (bind _character (Variables|Default|GetCharacter))
  ;[1 1 1] Set wwise switch depeing on physics material
  (switch Utilities|FlowControl|Switch|SwitchonEPhysicalSurface Selection
    (:SurfaceType_Default
      (Class|AkGameplayStatics|SetSwitch 0 _character "FootstepsSurface" "Default"))
    (:SurfaceType1
      (Class|AkGameplayStatics|SetSwitch 0 _character "FootstepsSurface" "Ice"))))

(event Custom|PlayDoubleJumpSound
  (if (== (Variables|/Game/_Game/Blueprints/Components/ParkourMovement.ParkourMovement_C|GetJumpCount (Variables|Default|GetParkourMovement)) 1)
    (Class|AkGameplayStatics|PostEvent "/Game/Audio/Events/Play_Double_Jump.Play_Double_Jump" (Variables|Default|GetCharacter))))

(event EventBeginPlay
  (Class|AkGameplayStatics|LoadBank "/Game/Audio/Soundbanks/PlayerSounds.PlayerSounds"))

(fn NewFunction0)
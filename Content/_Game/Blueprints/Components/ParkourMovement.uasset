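; Parkour movement component that adds wall running with camera tilt to a Character, set up through Initialize.
; A looping timer line-traces to each side and, while falling beside a valid wall, launches the character into and along it while easing gravity toward a target.
; Losing the wall restores default gravity and sets a timed suppression flag.
; Tick rolls the control rotation by wall side; jump and land events are empty.
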(event Custom|Initialize
  (params (Character :type Character%20Object%20Reference))
  (bind _output_get (Variables|Default|SetCharacter Character))
  (bind _output_get_2 (Variables|Default|SetCharacterMovment (Variables|/Script/Engine.Character|GetCharacterMovement _output_get)))
  (Variables|Default|SetDefaultGravityScale (Variables|/Script/Engine.CharacterMovementComponent|GetGravityScale _output_get_2))
  (Utilities|Time|SetTimerbyEvent (delegate Custom|Wallrun%20Update%20Event) 0.2 true))

(event Custom|Land%20Event)

(event Custom|Jump%20Event)

(event Custom|Wallrun%20Update%20Event
  (CallFunction|WallRunUpdate))

(event Custom|ResetWallRunSupression
  (Utilities|Time|ClearTimerbyFunctionName 0 "ResetWallRunSupression")
  (Variables|Default|SetWallRunSurpressed false))

(event EventBeginPlay)

(event EventTick
  (params (DeltaSeconds :type Float%20%28single-precision%29))
  (CallFunction|CameraTick))

(fn WallRunUpdate
  (bind _charactermovment (Variables|Default|GetCharacterMovment))
  (bind _onwall (CallFunction|WallRunMovement (Transformation|GetActorLocation (Variables|Default|GetCharacter)) (.Right (Utilities|WalRunEndVectors)) -1.0)) ; Right Side
  (if _onwall
    (bind _output_get (Variables|Default|SetWallRunning true))
    (Variables|Default|SetWallRunningOnRight _output_get)
    (Variables|Default|SetWallRunningOnLeft false)
    (Variables|/Script/Engine.CharacterMovementComponent|SetGravityScale _charactermovment (Math|Interpolation|FInterpTo (Variables|/Script/Engine.CharacterMovementComponent|GetGravityScale _charactermovment) (Variables|Default|GetWallRunTargetGravity) (Utilities|Time|GetWorldDeltaSeconds) 1e+01) :!label _label)
    (elif (Variables|Default|GetWallRunningOnRight)
      (CallFunction|WallRunEnd 1.0)
      (else
        (bind _onwall_2 (CallFunction|WallRunMovement (Transformation|GetActorLocation (Variables|Default|GetCharacter)) (.Left (Utilities|WalRunEndVectors)) 1.0)) ; Left Side
        (if _onwall_2
          (Variables|Default|SetWallRunning true)
          (Variables|Default|SetWallRunningOnRight false)
          (Variables|Default|SetWallRunningOnLeft true)
          (goto _label)
          (else
            (CallFunction|WallRunEnd 1.0)))))))

(fn WallRunMovement
  (params (Start :type Vector) (End :type Vector) (WallRunDirection :type Float%20%28double-precision%29))
  (bind _outhit (Collision|LineTraceByChannel Start End "TraceTypeQuery1" false 0 "None"))
  (if (.bblockinghit _outhit) ; Hit something?
    (Variables|Default|SetWallRunNormal (.OutVec (Utilities|ValidWallRunVector (.normal _outhit))))
    (if (and (AI|Components|NavMovement|IsFalling (Variables|Default|GetCharacterMovment)) (.ReturnValue (Utilities|ValidWallRunVector (.normal _outhit))))
      (Character|LaunchCharacter (Variables|Default|GetCharacter) (Utilities|PlayertoWallVector) false false) ; Stick Character to wall
      (Character|LaunchCharacter (Variables|Default|GetCharacter) (* (Math|Vector|CrossProduct (Variables|Default|GetWallRunNormal) "0, 0,1.000000") (* (Variables|Default|GetWallRunSpeed) WallRunDirection)) true (not (Variables|Default|GetWallRunGravity))) ; Move Character Forward
      (return true)
      (else
        (return false)))
    (else
      (return false))))

(fn WallRunEnd
  (params (Reset%20Time :type Float%20%28double-precision%29))
  (Variables|Default|SetWallRunning false)
  (Variables|Default|SetWallRunningOnRight false)
  (Variables|Default|SetWallRunningOnLeft false)
  (Variables|/Script/Engine.CharacterMovementComponent|SetGravityScale (Variables|Default|GetCharacterMovment) (Variables|Default|GetDefaultGravityScale))
  (CallFunction|SupressWallRun Reset%20Time))

(fn SupressWallRun
  (params (Delay :type Float%20%28double-precision%29))
  (Variables|Default|SetWallRunSurpressed true)
  (Utilities|Time|SetTimerbyFunctionName 0 "ResetWallRunSupression" Delay))

(fn CameraTick
  (if (Variables|Default|GetWallRunningOnLeft)
    (CallFunction|CameraTilt 15.0)
    (elif (Variables|Default|GetWallRunningOnRight)
      (CallFunction|CameraTilt -15.0)
      (else
        (CallFunction|CameraTilt 0.0)))))

(fn CameraTilt
  (params (Target%20X%20%28Roll%29 :type Float%20%28double-precision%29))
  (bind _character (Variables|Default|GetCharacter))
  (bind _returnvalue (Pawn|GetController _character))
  (bind _returnvalue_2 (Pawn|GetControlRotation _returnvalue :!class /Script/Engine.Controller))
  (bind (_roll _pitch _yaw) (Math|Rotator|BreakRotator _returnvalue_2))
  (Pawn|SetControlRotation _returnvalue (Math|Interpolation|RInterpTo _returnvalue_2 (Math|Rotator|MakeRotator Target%20X%20%28Roll%29 _pitch _yaw) (Utilities|Time|GetWorldDeltaSeconds) 1e+01)))
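; Actor component that lets its owning character pick up, carry and drop physics objects.
; Initialize caches the character and its first-person camera, which PickupObject line-traces from to grab a simulating component through the character's PhysicsHandle.
; Tick moves the handle target to the character's HeldObjectLocation, and DropObject releases it.
; The grab path still has debug trace drawing and a test print.
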(event Custom|Initialize
  (params (Character :type BP%20First%20Person%20Character%20Object%20Reference))
  (bind _output_get (Variables|Default|SetCharacter Character))
  (Variables|Default|SetFirst%20Person%20Camera%20Component (Variables|/Script/Unreal2022GameJam.Unreal2022GameJamCharacter|GetFirstPersonCameraComponent _output_get)))

(event Custom|PickupObject
  (bind _first_person_camera_component (Variables|Default|GetFirst%20Person%20Camera%20Component))
  (bind _returnvalue (Transformation|GetWorldLocation _first_person_camera_component))
  (bind (_outhit _returnvalue_2) (Collision|LineTraceByChannel _returnvalue (+ _returnvalue (* (Math|Vector|GetForwardVector _first_person_camera_component) (Variables|Default|GetGrabDistance))) "TraceTypeQuery1" false 0 "ForDuration"))
  (if _returnvalue_2
    (if (Physics|IsSimulatingPhysics (.hitcomponent _outhit) "None")
      (Development|PrintString "Hello")
      (Class|PhysicsHandleComponent|GrabComponentatLocation (Variables|/Game/FirstPerson/Blueprints/BP_FirstPersonCharacter.BP_FirstPersonCharacter_C|GetPhysicsHandle (Variables|Default|GetCharacter)) (.hitcomponent _outhit) "None" (Transformation|GetWorldLocation (.hitcomponent _outhit))))))

(event Custom|DropObject
  (Physics|Components|PhysicsHandle|ReleaseComponent (Variables|/Game/FirstPerson/Blueprints/BP_FirstPersonCharacter.BP_FirstPersonCharacter_C|GetPhysicsHandle (Variables|Default|GetCharacter))))

(event EventBeginPlay)

(event EventTick
  (params (DeltaSeconds :type Float%20%28single-precision%29))
  (Physics|Components|PhysicsHandle|SetTargetLocation (Variables|/Game/FirstPerson/Blueprints/BP_FirstPersonCharacter.BP_FirstPersonCharacter_C|GetPhysicsHandle (Variables|Default|GetCharacter)) (Transformation|GetWorldLocation (Variables|/Game/FirstPerson/Blueprints/BP_FirstPersonCharacter.BP_FirstPersonCharacter_C|GetHeldObjectLocation (Variables|Default|GetCharacter)))))
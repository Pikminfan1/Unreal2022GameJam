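; NewProjectile is a short-lived projectile that knocks the player character away on contact.
; It destroys itself after a LifeSpan delay, or on overlapping any actor other than a Turret_BP, which it ignores.
; On hitting a BP_PlayerCharacter, LaunchPlayer overrides the character's velocity with LaunchForce along LaunchDirection, rotated into the projectile's orientation and normalized.
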(event EventBeginPlay
  (Utilities|FlowControl|Delay (Variables|Default|GetLifeSpan))
  (Actor|DestroyActor))

(event Collision|EventActorBeginOverlap
  (params (OtherActor :type Actor%20Object%20Reference))
  (bind _asbp_player_character (Utilities|Casting|CastToBP_PlayerCharacter OtherActor)
    (:then
      (CallFunction|LaunchPlayer _asbp_player_character))
    (:CastFailed
      (Utilities|Casting|CastToTurret_BP OtherActor
        (:CastFailed
          _))))
  (Actor|DestroyActor self))

(event EventTick
  (params (DeltaSeconds :type Float%20%28single-precision%29)))

(fn ConstructionScript)

(fn LaunchPlayer
  (params (Player :type BP%20Player%20Character%20Object%20Reference))
  (Character|LaunchCharacter Player (* (Math|Vector|Normalize (Math|Vector|RotateVector (Variables|Default|GetLaunchDirection) (Transformation|GetActorRotation))) (Variables|Default|GetLaunchForce)) true true))
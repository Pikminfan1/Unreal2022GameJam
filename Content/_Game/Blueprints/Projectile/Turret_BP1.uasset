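; Turret actor that repeatedly fires ProjectileSphere_BP projectiles from its Arrow component's location and rotation.
; Tick feeds a DoOnce gate that spawns the projectile and posts a Wwise shot sound.
; After a FireRate delay, it plays the non-looping fire animation on the skeletal mesh and resets the gate, forming a continuous firing loop with no targeting logic.
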(event EventTick
  (params (DeltaSeconds :type Float%20%28single-precision%29))
  (bind _arrow (Variables|Default|GetArrow))
  (bind _returnvalue (Transformation|GetWorldTransform _arrow))
  (Utilities|FlowControl|DoOnce false :!label _label
    (:Completed
      (Game|SpawnActorfromClass "/Game/_Game/Blueprints/ProjectileSphere_BP.ProjectileSphere_BP_C" (Math|Transform|MakeTransform (.location _returnvalue) (.rotation _returnvalue)) "Undefined" 0 0)
      (Class|AkGameplayStatics|PostEvent "/Game/_Game/Audio/Events/Play_Turret_Shot.Play_Turret_Shot" self)
      (Utilities|FlowControl|Delay (Variables|Default|GetFireRate))
      (Components|Animation|PlayAnimation (Variables|Default|GetSkeletalMesh) "/Game/_Game/Characters/Animation/turret_anims/heaven_turret_fire_loop_v001_001.heaven_turret_fire_loop_v001_001" false)
      (goto _label Reset))))

(fn ConstructionScript
  (|CallParentFunction))
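; Projectile actor that knocks the player character away when it hits them, ignoring overlaps with turrets.
; On a player overlap it launches the character along its launch direction, rotated by the projectile's rotation and scaled by a force, overriding existing velocity.
; It destroys itself on any non-turret overlap or when its lifespan delay after BeginPlay expires.
; Toggle events are empty, and debug prints remain.
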(event Collision|EventActorBeginOverlap
  (params (OtherActor :type Actor%20Object%20Reference))
  (bind _asbp_player_character (Utilities|Casting|CastToBP_PlayerCharacter OtherActor)
    (:then
      (Development|PrintString "Hit Player")
      (CallFunction|LaunchPlayer _asbp_player_character))
    (:CastFailed
      (Utilities|Casting|CastToTurret_BP OtherActor
        (:CastFailed
          _))))
  (Actor|DestroyActor))

(event EventTick
  (params (DeltaSeconds :type Float%20%28single-precision%29)))

(event EventToggleon)

(event EventToggleOff)

(event EventBeginPlay
  (Utilities|FlowControl|Delay (Variables|Default|GetInitialLifeSpan))
  (Actor|DestroyActor))

(fn ConstructionScript
  (|CallParentFunction))

(fn LaunchPlayer
  (params (Player%20Character :type Unreal%202022%20Game%20Jam%20Character%20Object%20Reference))
  (bind _self self)
  (bind _launchdirection (Variables|Default|GetLaunchDirection))
  (bind _launchforce (Variables|Default|GetLaunchForce))
  (bind _returnvalue (Transformation|GetActorRotation _self))
  (bind _returnvalue_2 (Math|Vector|RotateVector _launchdirection _returnvalue))
  (bind _returnvalue_3 (Math|Vector|Normalize _returnvalue_2))
  (bind _returnvalue_4 (* _returnvalue_3 _launchforce))
  (Development|PrintString (Utilities|String|ToString(Vector) _returnvalue_4))
  (Character|LaunchCharacter Player%20Character _returnvalue_4 true true))